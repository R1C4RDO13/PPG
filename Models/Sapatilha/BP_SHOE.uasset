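; Shoe capture actor that automatically screenshots a shoe at random placements in original, red-vision and blue-vision variants.
; Each loop pass randomizes the shoe transform and camera position, with Tick keeping the camera aimed at the shoe.
; It cycles two post-process components between timed HighResShot console commands, saving each set under a shared GUID.
; Keys toggle the loop and view camera, reposition the scene or step the vision mode.
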(event Custom|TrigerNextCameraMode
  (bind _output_get (Variables|/Script/Engine.PostProcessComponent|SetbEnabled (Variables|Default|GetvisaoVermelha_proc) (Math|Boolean|NORBoolean (Variables|Default|GetVisaoVermelha_enabled) (Variables|Default|GetVisaoAzul_enabled))))
  (bind _output_get_2 (Variables|/Script/Engine.PostProcessComponent|SetbEnabled (Variables|Default|GetvisaoAzul_proc) (Variables|Default|GetVisaoVermelha_enabled)))
  (Variables|Default|SetVisaoAzul_enabled _output_get_2)
  (Variables|Default|SetVisaoVermelha_enabled _output_get))

(event Custom|TriggerNewPosition
  (Transformation|SetWorldLocationAndRotation (Variables|Default|Getshoe1) (Math|Random|RandomPointinBoundingBox (Transformation|GetWorldLocation (Variables|Default|GetDefaultSceneRoot)) (Variables|Default|GetHalfSize)) (Math|Random|RandomRotator false) false false)
  (Transformation|SetWorldLocation (Variables|Default|GetCamera) (Math|Random|RandomPointinBoundingBox (+ (Transformation|GetWorldLocation (Variables|Default|Getshoe1)) "0.000000,0.000000,100.000000") (Variables|Default|GetHalfSizeCamara)) false false)
  (Variables|Default|SetActivarFocoCamara true))

(event Custom|SwitchMainCamera
  (if (Variables|Default|GetCameraSelf)
    (Game|Player|SetViewTargetwithBlend (Game|GetPlayerController 0) (Game|Player|GetPlayerPawn 0) 0.0 "VTBlend_Linear" 0.5 false)
    (Variables|Default|SetCameraSelf false)
    (else
      (Game|Player|SetViewTargetwithBlend (Game|GetPlayerController 0) self 0.0 "VTBlend_Linear" 0.5 false)
      (Variables|Default|SetCameraSelf true))))

(event Custom|LOOP
  (if (Variables|Default|GetActivarFocoCamara)
    _
    (else
      (CallFunction|SwitchMainCamera)))
  (CallFunction|TriggerNewPosition)
  (Utilities|FlowControl|Delay 3.0)
  (Variables|Default|Setguid_current (Guid|ToString(Guid) (Guid|NewGuid)))
  (Variables|Default|Setmode_current "OG")
  (bind _output_get (Variables|Default|Setcommand (Utilities|String|ToString(Text) (Utilities|Text|FormatText "HighResShot 1920x1080 filename=\"c:/temp/img/image_{guid}_{mode_}.png\"" (Variables|Default|Getguid_current) (Variables|Default|Getmode_current)))))
  (Development|ExecuteConsoleCommand _output_get 0)
  (Utilities|FlowControl|Delay 0.02)
  (CallFunction|TrigerNextCameraMode)
  (Variables|Default|Setmode_current "RED")
  (bind _output_get_2 (Variables|Default|Setcommand (Utilities|String|ToString(Text) (Utilities|Text|FormatText "HighResShot 1920x1080 filename=\"c:/temp/img/image_{guid}_{mode_}.png\"" (Variables|Default|Getguid_current) (Variables|Default|Getmode_current)))))
  (Development|ExecuteConsoleCommand _output_get_2 0)
  (Utilities|FlowControl|Delay 0.02)
  (CallFunction|TrigerNextCameraMode)
  (Variables|Default|Setmode_current "BLUE")
  (bind _output_get_3 (Variables|Default|Setcommand (Utilities|String|ToString(Text) (Utilities|Text|FormatText "HighResShot 1920x1080 filename=\"c:/temp/img/image_{guid}_{mode_}.png\"" (Variables|Default|Getguid_current) (Variables|Default|Getmode_current)))))
  (Development|ExecuteConsoleCommand _output_get_3 0)
  (Utilities|FlowControl|Delay 0.02)
  (CallFunction|TrigerNextCameraMode)
  (Utilities|FlowControl|Delay 1.0)
  (if (Variables|Default|Getcontinue_loop)
    (CallFunction|LOOP)))

(event EventBeginPlay
  (Rendering|SetActorHiddenInGame (Game|Player|GetPlayerPawn 0) true)
  (Input|EnableInput (Game|GetPlayerController 0)))

(event Collision|EventActorBeginOverlap
  (params (OtherActor :type Actor%20Object%20Reference)))

(event EventTick
  (params (DeltaSeconds :type Float%20%28single-precision%29))
  (bind _camera (Variables|Default|GetCamera))
  (if (Variables|Default|GetActivarFocoCamara)
    (Transformation|SetWorldRotation _camera (Math|Rotator|FindLookatRotation (Transformation|GetWorldLocation _camera) (Transformation|GetWorldLocation (Variables|Default|Getshoe1))) false false)))

(event Input|KeyboardEvents|R
  (params (Key :type Key%20Structure :default "None"))
  (:Pressed
    (CallFunction|TriggerNewPosition)))

(event Input|KeyboardEvents|T
  (params (Key :type Key%20Structure :default "None"))
  (:Pressed
    (CallFunction|TrigerNextCameraMode)))

(event Input|KeyboardEvents|P
  (params (Key :type Key%20Structure :default "None"))
  (:Pressed
    (CallFunction|SwitchMainCamera)))

(event Input|KeyboardEvents|L
  (params (Key :type Key%20Structure :default "None"))
  (:Pressed
    (bind _output_get (Variables|Default|Setcontinue_loop (not (Variables|Default|Getcontinue_loop))))
    (if _output_get
      (CallFunction|LOOP))))

(fn ConstructionScript)